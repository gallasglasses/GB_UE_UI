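; Test actor for the save system that opens the WBP_SavingTest widget when its Interact event fires.
; BeginPlay stores the Sphere component's world location in InitialLocation, which nothing in this graph reads.
; Each Interact creates a new widget, stores it in SavingWidget and adds it to the viewport.
; The IsWidgetShowing toggle and widget removal nodes are disconnected, so this Blueprint never closes the widget.
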(event EventBeginPlay
  (Variables|Default|SetInitialLocation (Transformation|GetWorldLocation (Variables|Default|GetSphere))))

(event Collision|EventActorBeginOverlap
  (params (OtherActor :type Actor%20Object%20Reference)))

(event EventTick
  (params (DeltaSeconds :type Float%20%28single-precision%29)))

(event EventInteract
  (params (ActorInteractedWithObject :type Actor%20Object%20Reference))
  (bind _returnvalue (UserInterface|CreateWidget "/Game/HASGame/SaveSystem/WBP_SavingTest.WBP_SavingTest_C"))
  (Variables|Default|SetSavingWidget _returnvalue)
  (UserInterface|Viewport|AddtoViewport _returnvalue 0))

(fn ConstructionScript)